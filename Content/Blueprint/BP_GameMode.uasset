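; BP_GameMode is a game mode that shows the HUD and keeps timing state for a run.
; On BeginPlay it creates WBP_HUD, stores it in HUDWidget and adds it to the viewport.
; StartRunTimer records the game-time start and sets a running flag, while StopRunTimer stores the elapsed time as FinalTime, clears that flag and marks the game as ended.
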(event `self.ReceiveBeginPlay`
  (bind _returnvalue (`|CreateWidget` "/Game/Blueprint/WBP_HUD.WBP_HUD_C"))
  (bind _output_get (set `self.HUDWidget` _returnvalue))
  (`UserWidget.AddToViewport` _output_get 0))

(event `self.ReceiveTick`
  (params (DeltaSeconds :type "Float (single-precision)")))

(fn `StartRunTimer`
  (set `self.StartTime` (`KismetSystemLibrary.GetGameTimeInSeconds`))
  (set `self.bIsTimerRunning` true))

(fn `StopRunTimer`
  (set `self.FinalTime` (- (`KismetSystemLibrary.GetGameTimeInSeconds`) (`self.StartTime`)))
  (set `self.bIsTimerRunning` false)
  (set `self.bGameEnded` true))

(fn `UserConstructionScript`)