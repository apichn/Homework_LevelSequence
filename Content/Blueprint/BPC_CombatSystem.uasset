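; Combat component for an owner Character that plays random attack montages and applies melee hit damage.
; BeginAttackEvent blocks re-entry while attacking and broadcasts OnAttackFinish on completion or interruption, then EndAttackEvent clears the state and stops the stored montage.
; Hit trace functions sphere-sweep between a socket's previous and current positions, damaging each Pawn-type actor once per trace window, excluding the owner, with debug drawing on.
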(event `self.ReceiveBeginPlay`)

(event `BeginAttackEvent`
  (bind _outitem (`KismetArrayLibrary.Array_Random` (`self.AttackMontage`)))
  (if (not (`self.IsAttacking`))
    (`|PlayMontage` (`Character.Mesh` (`self.OwnerCharacter`)) _outitem
      (:`then`
        (`|ExecutionSequence`
          (:`then_0`
            (set `self.IsAttacking` true))
          (:`then_1`
            (set `self.LastAnimMontage` _outitem))))
      (:`OnCompleted`
        (`self.OnAttackFinish` true)
        (`self.EndAttackEvent` :!label _label))
      (:`OnInterrupted`
        (`self.OnAttackFinish` false)
        (goto _label)))))

(event `EndAttackEvent`
  (bind _lastanimmontage (`self.LastAnimMontage`))
  (`|ExecutionSequence`
    (:`then_0`
      (if (`self.IsAttacking`)
        (set `self.IsAttacking` false)))
    (:`then_1`
      (`/Engine/EditorBlueprintResources/StandardMacros.IsValid` _lastanimmontage
        (:`Is Valid`
          (`AnimInstance.Montage_Stop` (`SkeletalMeshComponent.GetAnimInstance` (`Character.Mesh` (`self.OwnerCharacter`))) 0.0 _lastanimmontage))))))

(fn `BeginHitTrace`
  (params (TraceSocketName :type Name))
  (set `self.TraceSocketName` TraceSocketName)
  (`KismetArrayLibrary.Array_Clear` (`self.HitActors`))
  (set `self.LastSocketLocation` (`SceneComponent.GetSocketLocation` (`Character.Mesh` (`self.OwnerCharacter`)) (`self.TraceSocketName`))))

(fn `EndhitTrace`
  (`KismetArrayLibrary.Array_Clear` (`self.HitActors`)))

(fn `GetOwnerCharacter`
  (returns (ReturnOwnerCharacter :type "/Game/ThirdPerson/Blueprints/BP_ThirdPersonCharacter Object Reference"))
  (return (`self.OwnerCharacter`)))

(fn `SetOwnerCharacter`
  (params (Character :type "/Game/ThirdPerson/Blueprints/BP_ThirdPersonCharacter Object Reference"))
  (set `self.OwnerCharacter` Character))

(fn `TickHitTrace`
  (locals (Current :type "Vector Structure" :default (0.0 0.0 0.0)))
  (bind _ownercharacter (`self.OwnerCharacter`))
  (bind _hitactors (`self.HitActors`))
  (bind _output_get (set `local.Current` (`SceneComponent.GetSocketLocation` (`Character.Mesh` (`self.OwnerCharacter`)) (`self.TraceSocketName`))))
  (bind _outhits (`KismetSystemLibrary.SphereTraceMultiForObjects` :`Start` (`self.LastSocketLocation`) :`End` _output_get :`Radius` (`self.TraceRadius`) :`ObjectTypes` (`|MakeArray` "ObjectTypeQuery3" :!type "EObjectTypeQuery Enum") :`DrawDebugType` "ForDuration" :`DrawTime` 0.2))
  (for _array_element _outhits
    (bind (_bblockinghit _binitialoverlap _time _distance _location _impactpoint _normal _impactnormal _physmat _hitactor) (`GameplayStatics.BreakHitResult` _array_element))
    (if (and (!= _hitactor _ownercharacter) (not (`KismetArrayLibrary.Array_Contains` _hitactors _hitactor)))
      (`KismetArrayLibrary.Array_AddUnique` _hitactors _hitactor)
      (`GameplayStatics.ApplyDamage` _hitactor (`self.AttackDamage`) (`Pawn.GetController` _ownercharacter) (`self.GetOwner`) "/Script/Engine.DamageType")))
  (set `self.LastSocketLocation` (`local.Current`)))