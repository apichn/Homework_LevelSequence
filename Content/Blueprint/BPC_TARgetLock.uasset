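; Target lock component for BP_PlayerCharacter that searches for a lock target and feeds it to the GameplayCamera rig.
; SetFindTarget starts or clears a looping timer for the periodic search and sets the rig's lock-on parameters.
; FindClosetTarget sphere-traces around the player, keeping the last targetable hit without comparing distances; Istargetable is a stub returning false.
; A valid target sets the camera's lock direction; otherwise that vector is zeroed.
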(event `self.ReceiveBeginPlay`
  (bind _asbp_player_character (cast `/Game/ThirdPerson/Blueprints/BP_PlayerCharacter` (`self.GetOwner`)))
  (set `self.As BP PlayerCharacter` _asbp_player_character)
  (`self.SetFindTarget` false))

(event `FindTargetEvent`
  (bind _gameplaycamera (`/Game/ThirdPerson/Blueprints/BP_PlayerCharacter.GameplayCamera` (`self.As BP PlayerCharacter`)))
  (bind _returnvalue (`GameplayCameraComponentBase.GetInitialResult` _gameplaycamera))
  (if (`self.IsFinding`)
    (set `self.LockTarget` (`self.FindClosetTarget`))
    (`/Engine/EditorBlueprintResources/StandardMacros.IsValid` null
      (:`Is Valid`
        (`|SetCameraRigParameter` _returnvalue (- (`Actor.K2_GetActorLocation` (`self.LockTarget`)) (`SceneComponent.K2_GetComponentLocation` _gameplaycamera)))
        (`|SetCameraRigParameter` _returnvalue true))
      (:`Is Not Valid`
        (`|SetCameraRigParameter` _returnvalue true)
        (`|SetCameraRigParameter` _returnvalue)))))

(fn `FindClosetTarget`
  (returns (ReturnTarget :type "Actor Object Reference"))
  (locals (Closest :type "Actor Object Reference"))
  (bind _returnvalue (`Actor.K2_GetActorLocation` (`self.As BP PlayerCharacter`)))
  (bind (_outhits _returnvalue_2) (`KismetSystemLibrary.SphereTraceMultiForObjects` :`Start` _returnvalue :`End` _returnvalue :`Radius` 500.0 :`ObjectTypes` (`self.Object Types`) :`DrawDebugType` "ForOneFrame"))
  (if _returnvalue_2
    (for _array_element _outhits
      (bind _isable (`self.Istargetable`))
      (if _isable
        (set `local.Closest` (`.HitActor` (`GameplayStatics.BreakHitResult` _array_element))))))
  (return (`local.Closest`)))

(fn `Istargetable`
  (returns (Isable :type Boolean))
  (return false))

(fn `NewFunction`)

(fn `SetFindTarget`
  (params (IsFinding :type Boolean))
  (bind _returnvalue (`GameplayCameraComponentBase.GetInitialResult` (`/Game/ThirdPerson/Blueprints/BP_PlayerCharacter.GameplayCamera` (`self.As BP PlayerCharacter`))))
  (bind _output_get (set `self.IsFinding` IsFinding))
  (if _output_get
    (bind _returnvalue_2 (`KismetSystemLibrary.K2_SetTimerDelegate` (`|CreateDelegate` :!event `FindTargetEvent`) 0.2 true))
    (set `self.FindTargetTime` _returnvalue_2)
    (`|SetCameraRigParameter` _returnvalue true)
    (`|SetCameraRigParameter` _returnvalue)
    (else
      (`KismetSystemLibrary.K2_ClearAndInvalidateTimerHandle` (`self.FindTargetTime`))
      (set `self.LockTarget` null))))