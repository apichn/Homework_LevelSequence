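; Health component that tracks current and maximum health and a dead state for its owner.
; InitHealth fills health to the given maximum, and DecreaseHealth clamps damage at zero, both broadcasting a health update.
; A guard flag makes the death event fire only once when health runs out.
; IncreaseHealth caps healing at the maximum without broadcasting, and GetIsDead is an empty stub.
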(fn `DecreaseHealth`
  (params (Value :type "Float (double-precision)"))
  (bind _health (`self.Health`))
  (if (> _health 0.0)
    (bind _output_get (set `self.Health` (`KismetMathLibrary.FMax` (- _health Value))))
    (`self.OnHealthUpdate` _output_get (`self.MaxHealth`))
    (if (and (>= 0.0 (`self.Health`)) (not (`self.IsDead`)))
      (set `self.IsDead` true)
      (`self.OnDeath`))))

(fn `GetHealth`
  (returns (ReturnHealth :type "Float (double-precision)"))
  (return (`self.Health`)))

(fn `GetIsDead`)

(fn `GetMaxHealth`
  (returns (ReturnHealth :type "Float (double-precision)"))
  (return (`self.MaxHealth`)))

(fn `InCreaseHealth`
  (params (Value :type "Float (double-precision)"))
  (set `self.Health` (`KismetMathLibrary.FMin` (`self.MaxHealth`) (+ (`self.Health`) Value))))

(fn `InitHealth`
  (params (MaxHealth :type "Float (double-precision)"))
  (bind _output_get (set `self.MaxHealth` MaxHealth))
  (bind _output_get_2 (set `self.Health` _output_get))
  (`self.OnHealthUpdate` _output_get_2 _output_get))