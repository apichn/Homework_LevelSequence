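; BP_VictoryTrigger is a one-shot trigger volume that ends the run with a win when the player reaches it.
; On the first overlap of its Collision by the player pawn, it marks itself used and tells BP_GameMode to stop the run timer.
; It then shows the WBP_Win widget and plays an attached Actor Sequence.
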(event `self.collision.OnComponentBeginOverlap`
  (params (OverlappedComponent :type "PrimitiveComponent Object Reference") (OtherActor :type "Actor Object Reference") (OtherComp :type "PrimitiveComponent Object Reference") (OtherBodyIndex :type Integer) (bFromSweep :type Boolean) (SweepResult :type "HitResult Structure (by ref)"))
  (if (and (not (`self.IsUsed`)) (== (`GameplayStatics.GetPlayerPawn` 0) OtherActor))
    (set `self.IsUsed` true)
    (bind _asbp_game_mode (cast `/Game/Blueprint/BP_GameMode` (`GameplayStatics.GetGameMode`)))
    (`/Game/Blueprint/BP_GameMode.StopRunTimer` _asbp_game_mode)
    (`|ExecutionSequence`
      (:`then_0`
        (bind _returnvalue (`|CreateWidget` "/Game/Blueprint/WBP_Win.WBP_Win_C" (`GameplayStatics.GetPlayerController` 0)))
        (`UserWidget.AddToViewport` _returnvalue 0))
      (:`then_1`
        (`ActorSequenceComponent.PlaySequence` (`self.ActorSequence`))))))

(fn `UserConstructionScript`)