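; Camera director for the player that picks which camera rig is active in the Gameplay Camera system.
; Each evaluation reads the CameraStyle gameplay tag from the owning BP_PlayerCharacter and branches with hierarchical tag matching.
; Third-person styles use the free or lock rig, first-person uses its own rig, and any other style falls back to the fixed camera rig.
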(event `self.RunCameraDirector`
  (params (DeltaTime :type "Float (single-precision)") (EvaluationContextOwner :type "Object Object Reference") (Params :type "BlueprintCameraDirectorEvaluationParams Structure (by ref)"))
  (bind _camerastyle (`/Game/ThirdPerson/Blueprints/BP_PlayerCharacter.CameraStyle` (`self.FindEvaluationContextOwnerActor` "/Game/ThirdPerson/Blueprints/BP_PlayerCharacter.BP_PlayerCharacter_C")))
  (if (`BlueprintGameplayTagLibrary.MatchesTag` _camerastyle (struct :`TagName` "Camera.Style.TPS"))
    (if (`BlueprintGameplayTagLibrary.MatchesTag` _camerastyle (struct :`TagName` "Camera.Style.TPS.NoLock"))
      (`self.ActivateCameraRig` "/Game/Blueprint/CR_Thirdperson.CR_Thirdperson")
      (else
        (`self.ActivateCameraRig` "/Game/Blueprint/CR_Thirdperson_Lock.CR_Thirdperson_Lock")))
    (elif (`BlueprintGameplayTagLibrary.MatchesTag` _camerastyle (struct :`TagName` "Camera.Style.FPS"))
      (`self.ActivateCameraRig` "/Game/Blueprint/CR_FirstPerson.CR_FirstPerson")
      (else
        (`self.ActivateCameraRig` "/Game/Blueprint/CR_FixCamera.CR_FixCamera")))))